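; Wind hazard zone controller that starts repeating gusts when the Hero enters BeginWindZone and stops scheduling them after EndWindZone is overlapped.
; Each cycle waits randomly, plays a warning sound, then runs a damage step meant to zero WarmValue outside SafeZone.
; As wired, DamagedFromThisGust is never cleared, so damage never applies.
; The counter check ends each gust after one tick, and both wind stages only zero the Hero's wind rotations.
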(event `self.Begin Wind Zone.OnComponentBeginOverlap`
  (params (OverlappedComponent :type "PrimitiveComponent Object Reference") (OtherActor :type "Actor Object Reference") (OtherComp :type "PrimitiveComponent Object Reference") (OtherBodyIndex :type Integer) (bFromSweep :type Boolean) (SweepResult :type "HitResult Structure (by ref)"))
  (bind _damage_counter (`self.Damage Counter`))
  (bind _ashero (cast `/Game/Blueprints/FirstPerson/Hero` OtherActor))
  (bind _output_get (set `self.On/Off` true))
  (if _output_get :!label _label
    (`KismetSystemLibrary.RetriggerableDelay` (`KismetMathLibrary.RandomFloatInRange` 10.0 30.0))
    (set `self.Damaged from this gust` true)
    (`self.stage 1 wind` _ashero)
    (`KismetSystemLibrary.Delay` 3.0)
    (set `self.Damage Counter` 0.0)
    (`KismetSystemLibrary.RetriggerableDelay` 0.01 :!label _label_2)
    (`self.damaging wind` _ashero)
    (`/Engine/EditorBlueprintResources/StandardMacros.IncrementFloat` _damage_counter
      (:`  `
        (if (> _damage_counter 200.0)
          (goto _label_2)
          (else
            (`self.return to normal` _ashero)
            (goto _label)))))))

(event `self.End Wind Zone.OnComponentBeginOverlap`
  (params (OverlappedComponent :type "PrimitiveComponent Object Reference") (OtherActor :type "Actor Object Reference") (OtherComp :type "PrimitiveComponent Object Reference") (OtherBodyIndex :type Integer) (bFromSweep :type Boolean) (SweepResult :type "HitResult Structure (by ref)"))
  (set `self.On/Off` false))

(event `self.Safe Zone.OnComponentBeginOverlap`
  (params (OverlappedComponent :type "PrimitiveComponent Object Reference") (OtherActor :type "Actor Object Reference") (OtherComp :type "PrimitiveComponent Object Reference") (OtherBodyIndex :type Integer) (bFromSweep :type Boolean) (SweepResult :type "HitResult Structure (by ref)"))
  (set `self.Player In Safe Zone` true))

(event `self.Safe Zone.OnComponentEndOverlap`
  (params (OverlappedComponent :type "PrimitiveComponent Object Reference") (OtherActor :type "Actor Object Reference") (OtherComp :type "PrimitiveComponent Object Reference") (OtherBodyIndex :type Integer))
  (set `self.Player In Safe Zone` false))

(fn `damaging wind`
  (params (Hero :type "/Game/Blueprints/FirstPerson/Hero Object Reference"))
  (if (`self.Player In Safe Zone`)
    _
    (elif (not (`self.Damaged from this gust`))
      (set `self.Damaged from this gust` true)
      (set `/Game/Blueprints/FirstPerson/Hero.WarmValue` 0 Hero))))

(fn `return to normal`
  (params (Hero :type "/Game/Blueprints/FirstPerson/Hero Object Reference"))
  (set `/Game/Blueprints/FirstPerson/Hero.Wind X Rotation` 0.0 Hero)
  (set `/Game/Blueprints/FirstPerson/Hero.Wind Y Rotation` 0.0 Hero))

(fn `stage 1 wind`
  (params (Hero :type "/Game/Blueprints/FirstPerson/Hero Object Reference"))
  (`GameplayStatics.PlaySoundAtLocation` null (`SceneComponent.K2_GetComponentLocation` (`Character.CapsuleComponent` Hero)) (struct) 1.0 1.0 0.0 null null null)
  (set `/Game/Blueprints/FirstPerson/Hero.Wind X Rotation` 0.0 Hero)
  (set `/Game/Blueprints/FirstPerson/Hero.Wind Y Rotation` 0.0 Hero))

(fn `UserConstructionScript`)