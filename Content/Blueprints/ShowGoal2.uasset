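; ShowGoal2 is a trigger actor that marks the player's first goal complete and switches the HUD to the second goal.
; Any overlap on its StaticMesh checks the player Hero's FulfillGoal1 flag, without checking which actor overlapped.
; If the flag is unset, it sets it and calls Goal2 on the MainWidgetHud held by MainHUD, so the change happens only once.
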(event `self.StaticMesh.OnComponentBeginOverlap`
  (params (OverlappedComponent :type "PrimitiveComponent Object Reference") (OtherActor :type "Actor Object Reference") (OtherComp :type "PrimitiveComponent Object Reference") (OtherBodyIndex :type Integer) (bFromSweep :type Boolean) (SweepResult :type "HitResult Structure (by ref)"))
  (bind _ashero (cast `/Game/Blueprints/FirstPerson/Hero` (`GameplayStatics.GetPlayerCharacter` 0)))
  (if (not (`/Game/Blueprints/FirstPerson/Hero.FulfillGoal1` _ashero))
    (set `/Game/Blueprints/FirstPerson/Hero.FulfillGoal1` true _ashero)
    (bind _asmain_hud (cast `/Game/Blueprints/FirstPerson/MainHUD` (`PlayerController.GetHUD` (`GameplayStatics.GetPlayerController` 0))))
    (bind _asmain_widget_hud (cast `/Game/Blueprints/FirstPerson/MainWidgetHud` (`/Game/Blueprints/FirstPerson/MainHUD.MainWidgetValue` _asmain_hud)))
    (`/Game/Blueprints/FirstPerson/MainWidgetHud.Goal2` _asmain_widget_hud)))

(fn `UserConstructionScript`)