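; FogControl drives a blizzard fog zone, using two overlap triggers to fade exponential height fog in and out and toggle the Hero's weather flags.
; The fade-in trigger gradually thickens the fog through a RetriggerableDelay loop, then pulses it on a modulo cycle via FogMovement.
; The fade-out trigger sets FadeOut to break that loop and thins the fog faster.
; IncreaseDensity caps density, while DecreaseDensity snaps it to zero near the minimum.
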(event `self.Fog Fade In Trigger.OnComponentBeginOverlap`
  (params (OverlappedComponent :type "PrimitiveComponent Object Reference") (OtherActor :type "Actor Object Reference") (OtherComp :type "PrimitiveComponent Object Reference") (OtherBodyIndex :type Integer) (bFromSweep :type Boolean) (SweepResult :type "HitResult Structure (by ref)"))
  (bind _periodofdensitychange (`self.PeriodOfDensityChange`))
  (bind _movementcounter (`self.MovementCounter`))
  (bind _ashero (cast `/Game/Blueprints/FirstPerson/Hero` OtherActor))
  (set `/Game/Blueprints/FirstPerson/Hero.BlizzardEnable` true _ashero)
  (set `self.MovementCounter` 0)
  (`KismetSystemLibrary.RetriggerableDelay` _periodofdensitychange :!label _label)
  (if (not (`self.FadeOut`))
    (`self.Increase Density` 0.0025)
    (bind _result (`/Engine/EditorBlueprintResources/StandardMacros.IncrementInt` _movementcounter)
      (:`  `
        (if (< _result 800)
          (goto _label)
          (else
            (`KismetSystemLibrary.PrintString` (`KismetStringLibrary.Conv_ObjectToString` _ashero))
            (`self.Fog Movement` _movementcounter :!label _label_2)
            (`/Engine/EditorBlueprintResources/StandardMacros.IncrementInt` _movementcounter
              (:`  `
                (`KismetSystemLibrary.RetriggerableDelay` _periodofdensitychange)
                (if (not (`self.FadeOut`))
                  (goto _label_2))))))))))

(event `self.Fog Fade Out Trigger.OnComponentBeginOverlap`
  (params (OverlappedComponent :type "PrimitiveComponent Object Reference") (OtherActor :type "Actor Object Reference") (OtherComp :type "PrimitiveComponent Object Reference") (OtherBodyIndex :type Integer) (bFromSweep :type Boolean) (SweepResult :type "HitResult Structure (by ref)"))
  (bind _movementcounter (`self.MovementCounter`))
  (set `/Game/Blueprints/FirstPerson/Hero.BlizzardEnable` false (stale `self.Fog Fade In Trigger.OnComponentBeginOverlap` _ashero))
  (set `/Game/Blueprints/FirstPerson/Hero.SnowEnable` false (stale `self.Fog Fade In Trigger.OnComponentBeginOverlap` _ashero))
  (set `self.FadeOut` true)
  (set `self.MovementCounter` 0)
  (`KismetSystemLibrary.RetriggerableDelay` (/ (`self.PeriodOfDensityChange`) 4.0) :!label _label_3)
  (`self.Decrease Density` 0.02)
  (`/Engine/EditorBlueprintResources/StandardMacros.IncrementInt` _movementcounter
    (:`  `
      (if (< _movementcounter 100)
        (goto _label_3)))))

(fn `Decrease Density`
  (params (Amount :type "Float (double-precision)"))
  (bind _exponentialheightfog (`self.ExponentialHeightFog`))
  (bind _fogdensity (`ExponentialHeightFogComponent.FogDensity` _exponentialheightfog))
  (`ExponentialHeightFogComponent.SetFogDensity` _exponentialheightfog (- _fogdensity Amount))
  (bind _output_get (set `self.MinFogDensity` 0.01))
  (if (not (> _fogdensity _output_get))
    (`ExponentialHeightFogComponent.SetFogDensity` (`self.ExponentialHeightFog`) 0.0)))

(fn `Fog Movement`
  (params (Iteration :type Integer))
  (`/Engine/EditorBlueprintResources/StandardMacros.CompareInt` (mod Iteration 800) 200
    (:`>`
      (`self.Increase Density` 0.0075))
    (:`<`
      (`self.Decrease Density` 0.0075))))

(fn `Increase Density`
  (params (Amount :type "Float (double-precision)"))
  (bind _exponentialheightfog (`self.ExponentialHeightFog`))
  (bind _fogdensity (`ExponentialHeightFogComponent.FogDensity` _exponentialheightfog))
  (`ExponentialHeightFogComponent.SetFogDensity` _exponentialheightfog (+ _fogdensity Amount))
  (bind _output_get (set `self.MaxFogDensity` 2.0))
  (if (not (> _output_get _fogdensity))
    (`ExponentialHeightFogComponent.SetFogDensity` (`self.ExponentialHeightFog`) _output_get)))

(fn `UserConstructionScript`)