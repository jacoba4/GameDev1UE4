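; MainMenuHUD is a HUD Blueprint that shows the correct screen for the main menu and the game's ending levels.
; On BeginPlay it enables the mouse cursor, then compares the current level name against Menu, BadEnding and GoodEnding.
; A match creates the corresponding main menu, bad ending or good ending widget and adds it to the viewport.
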(event `self.ReceiveBeginPlay`
  (set `PlayerController.bShowMouseCursor` true (`GameplayStatics.GetPlayerController` 0))
  (bind _returnvalue (`GameplayStatics.GetCurrentLevelName` true))
  (if (`KismetStringLibrary.EqualEqual_StrStr` _returnvalue "Menu")
    (bind _returnvalue_2 (`|CreateWidget` "/Game/Blueprints/MainMenu/MainMenuWidget.MainMenuWidget_C"))
    (`UserWidget.AddToViewport` _returnvalue_2 0)
    (elif (`KismetStringLibrary.EqualEqual_StrStr` _returnvalue "BadEnding")
      (bind _returnvalue_3 (`|CreateWidget` "/Game/Blueprints/MainMenu/BadEndingWidget.BadEndingWidget_C"))
      (`UserWidget.AddToViewport` _returnvalue_3 0)
      (elif (`KismetStringLibrary.EqualEqual_StrStr` _returnvalue "GoodEnding")
        (bind _returnvalue_4 (`|CreateWidget` "/Game/Blueprints/MainMenu/GoodEndingWidget.GoodEndingWidget_C"))
        (`UserWidget.AddToViewport` _returnvalue_4 0)))))

(fn `UserConstructionScript`)