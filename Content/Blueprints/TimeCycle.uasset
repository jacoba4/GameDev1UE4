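; Time-of-day controller that advances the sun as the Hero gets closer to the Tower than ever before.
; Delayed Tick turns closest-distance progress, relative to the starting distance, into incremental Light pitch rotations and updates BP_Sky_Sphere.
; A pitch threshold flags night to change disabled light-function brightness, though this casts the Light actor to LightComponent.
; PrevFrameNight always becomes true on a change, so it does not truly track the previous state.
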(event `self.ReceiveBeginPlay`
  (bind _returnvalue (`Actor.GetDistanceTo` (`self.Player`) (`self.Tower`)))
  ;[1 1 1] Player-Tower Distance
  (`KismetSystemLibrary.Delay` 0.2)
  (bind _outactors (`GameplayStatics.GetAllActorsWithTag` "Hero"))
  (set `self.Player` (`|GetArrayItem` _outactors))
  (bind _outactors_2 (`GameplayStatics.GetAllActorsWithTag` "Tower"))
  (set `self.Tower` (`|GetArrayItem` _outactors_2))
  (set `self.MinDistance` _returnvalue)
  (set `self.MaxDistance` _returnvalue)
  (bind _outactors_3 (`GameplayStatics.GetAllActorsWithTag` "SkySphere"))
  (bind _asbp_sky_sphere (cast `/Engine/EngineSky/BP_Sky_Sphere` (`|GetArrayItem` _outactors_3)))
  (set `self.SkySphere` _asbp_sky_sphere))

(event `self.ReceiveTick`
  (params (DeltaSeconds :type "Float (single-precision)"))
  (bind _maxdistance (`self.MaxDistance`))
  (bind _night (`self.Night`))
  (bind _light (`self.Light`))
  (bind _light_2 (`self.Light`))
  (bind _returnvalue (!= (`self.PrevFrameNight`) _night))
  (bind _returnvalue_2 (/ (- _maxdistance (`self.MinDistance`)) _maxdistance))
  (`KismetSystemLibrary.Delay` 0.2)
  (bind _output_get (set `self.PlayerTowerDistance` (`Actor.GetDistanceTo` (`self.Player`) (`self.Tower`))))
  (`/Engine/EditorBlueprintResources/StandardMacros.CompareFloat` _output_get (`self.MinDistance`)
    (:`>`
      _)
    (:`==`
      _)
    (:`<`
      (set `self.MinDistance` _output_get)))
  (`/Engine/EditorBlueprintResources/StandardMacros.CompareFloat` _returnvalue_2 (`self.MaxProgress`)
    (:`>`
      (bind _output_get_2 (set `self.MaxProgress` _returnvalue_2))
      (`Actor.K2_AddActorLocalRotation` _light_2 (`KismetMathLibrary.MakeRotator` 0.0 (* _output_get_2 7.0)) false false)
      (`/Engine/EngineSky/BP_Sky_Sphere.UpdateSunDirection` (`self.SkySphere`)))
    (:`==`
      _)
    (:`<`
      _))
  (set `self.Night` (`KismetMathLibrary.InRange_FloatFloat` (.pitch (`Actor.K2_GetActorRotation` _light_2)) (`self.NightThreshold`) 100.0))
  (if _returnvalue
    (set `self.PrevFrameNight` _returnvalue)
    (if _night
      (`KismetSystemLibrary.PrintString` "Good Night")
      (bind _aslight_component (cast `LightComponent` _light))
      (`LightComponent.SetLightFunctionDisabledBrightness` _aslight_component 0.0)
      (else
        (`KismetSystemLibrary.PrintString` "Good Night")
        (bind _aslight_component_2 (cast `LightComponent` _light))
        (`LightComponent.SetLightFunctionDisabledBrightness` _aslight_component_2 3.141593)))))