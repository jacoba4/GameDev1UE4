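; Snowdrift actor that flags the player Hero as being in a snowdrift and lowers their camera while its volumes are overlapped.
; Begin overlap on the Cylinder or Sphere sets IsSnowdrift and shifts HeroCamera down locally; end overlap clears the flag and shifts it back up.
; Handlers act on player character 0 without checking the overlapping actor, and the relative offsets can stack across both volumes.
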(event `self.Cylinder.OnComponentBeginOverlap`
  (params (OverlappedComponent :type "PrimitiveComponent Object Reference") (OtherActor :type "Actor Object Reference") (OtherComp :type "PrimitiveComponent Object Reference") (OtherBodyIndex :type Integer) (bFromSweep :type Boolean) (SweepResult :type "HitResult Structure (by ref)"))
  (bind _ashero (cast `/Game/Blueprints/FirstPerson/Hero` (`GameplayStatics.GetPlayerCharacter` 0) :!label _label))
  (set `/Game/Blueprints/FirstPerson/Hero.IsSnowdrift` true _ashero)
  (`SceneComponent.K2_AddLocalTransform` (`/Game/Blueprints/FirstPerson/Hero.HeroCamera` _ashero) (`KismetMathLibrary.MakeTransform` (0.0 0.0 -50.0)) false false))

(event `self.Sphere.OnComponentBeginOverlap`
  (params (OverlappedComponent :type "PrimitiveComponent Object Reference") (OtherActor :type "Actor Object Reference") (OtherComp :type "PrimitiveComponent Object Reference") (OtherBodyIndex :type Integer) (bFromSweep :type Boolean) (SweepResult :type "HitResult Structure (by ref)"))
  (goto _label))

(event `self.Cylinder.OnComponentEndOverlap`
  (params (OverlappedComponent :type "PrimitiveComponent Object Reference") (OtherActor :type "Actor Object Reference") (OtherComp :type "PrimitiveComponent Object Reference") (OtherBodyIndex :type Integer))
  (bind _ashero (cast `/Game/Blueprints/FirstPerson/Hero` (`GameplayStatics.GetPlayerCharacter` 0) :!label _label_2))
  (set `/Game/Blueprints/FirstPerson/Hero.IsSnowdrift` false _ashero)
  (`SceneComponent.K2_AddLocalTransform` (`/Game/Blueprints/FirstPerson/Hero.HeroCamera` _ashero) (`KismetMathLibrary.MakeTransform` (0.0 0.0 50.0)) false false))

(event `self.Sphere.OnComponentEndOverlap`
  (params (OverlappedComponent :type "PrimitiveComponent Object Reference") (OtherActor :type "Actor Object Reference") (OtherComp :type "PrimitiveComponent Object Reference") (OtherBodyIndex :type Integer))
  (goto _label_2))

(fn `UserConstructionScript`)